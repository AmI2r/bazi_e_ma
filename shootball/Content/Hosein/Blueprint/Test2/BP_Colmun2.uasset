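; BP_Colmun2 is a test column actor that bobs its cylinder mesh vertically in world space.
; Each Tick moves the mesh one unit up or down according to the Direction flag, so speed depends on frame rate.
; Direction flips to descending once world Z rises above zero, and back to ascending once it drops to the Loc variable or below.
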(event `self.ReceiveTick`
  (params (DeltaSeconds :type "Float (single-precision)"))
  (bind _shootball_test2_pcylinder6 (`self.Shootball_test2_pCylinder6`))
  (bind (_returnvalue_x _returnvalue_y _returnvalue_z) (`KismetMathLibrary.BreakVector` (`SceneComponent.K2_GetComponentLocation` _shootball_test2_pcylinder6)))
  (bind (_returnvalue_x_2 _returnvalue_y_2 _returnvalue_z_2) (`KismetMathLibrary.BreakVector` (`SceneComponent.K2_GetComponentLocation` (`self.Shootball_test2_pCylinder6`))))
  (bind (_returnvalue_x_3 _returnvalue_y_3 _returnvalue_z_3) (`KismetMathLibrary.BreakVector` (`SceneComponent.K2_GetComponentLocation` (`self.Shootball_test2_pCylinder6`))))
  (bind (_returnvalue_x_4 _returnvalue_y_4 _returnvalue_z_4) (`KismetMathLibrary.BreakVector` (`SceneComponent.K2_GetComponentLocation` _shootball_test2_pcylinder6)))
  (if (`self.Direction`)
    (`SceneComponent.K2_SetWorldLocation` _shootball_test2_pcylinder6 (`KismetMathLibrary.MakeVector` _returnvalue_x_4 _returnvalue_y_4 (+ _returnvalue_z_4 1.0)) false false)
    (if (not (<= _returnvalue_z_2 0.0))
      (set `self.Direction` false))
    (else
      (`SceneComponent.K2_SetWorldLocation` _shootball_test2_pcylinder6 (`KismetMathLibrary.MakeVector` _returnvalue_x _returnvalue_y (+ _returnvalue_z -1.0)) false false)
      (if (>= (`self.loc`) _returnvalue_z_3)
        (set `self.Direction` true)))))

(event `self.ReceiveBeginPlay`)

(fn `UserConstructionScript`)